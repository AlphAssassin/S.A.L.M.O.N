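; Player state for the free-for-all mode, holding a player's name and replicated kill and death stats.
; On BeginPlay the server polls each tick until the owning first-person controller's profile has loaded, then copies the player name from it.
; The kills RepNotify refreshes the scoreboard through the local controller's HUD widget, while the profile and deaths notifies are empty.
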(event `self.ReceiveCopyProperties`
  (params (NewPlayerState :type "PlayerState Object Reference")))

(event `self.ReceiveBeginPlay`
  (if (`KismetSystemLibrary.IsServer`)
    (bind _asbp_first_person_controller (cast `/Game/_Main/Game/Blueprints/Controllers/BP_FirstPersonController` (`self.GetPlayerController`)))
    (bind _output_get (set `self.BP First Person Controller` _asbp_first_person_controller))
    (if (`/Game/_Main/Game/Blueprints/Controllers/BP_FirstPersonController.isProfiledLoaded` _output_get) :!label _label
      (bind _output_get_2 (set `self.S Player Profile` (`/Game/_Main/Game/Blueprints/Controllers/BP_FirstPersonController.S Player Profile` _output_get)))
      (set `self.My Player Name` (`.PlayerName_2_EB8B0EAE472EF0E8B03D6C9F55C6C98E` (break `/Game/_Main/PlayerName/S_PlayerProfile` _output_get_2)))
      (else
        (`KismetSystemLibrary.DelayUntilNextTick`)
        (goto _label)))))

(fn `OnRep_Deaths`)

(fn `OnRep_Kills`
  (bind _asbp_first_person_controller (cast `/Game/_Main/Game/Blueprints/Controllers/BP_FirstPersonController` (`GameplayStatics.GetPlayerController` 0))
    (:`then`
      (`/Game/_Main/Game/Blueprints/Widgets/WBP_Hud.Update Scoreboard` (`/Game/_Main/Game/Blueprints/Controllers/BP_FirstPersonController.HudWidget` _asbp_first_person_controller)))
    (:`CastFailed`
      (`KismetSystemLibrary.PrintString` "Failed to update scoreboard"))))

(fn `OnRep_PlayerProfile`)

(fn `UserConstructionScript`)