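; Free-for-all game mode that starts the match countdown and picks respawn points.
; BeginPlay copies score limit, duration and player count from the lobby GameInstance; Server_PlayerReady counts players, polling until that count is nonzero, then starts every controller's countdown when all are ready.
; Respawn returns the PlayerStart with the largest distance to any single living player, not the farthest from the nearest.
; Session-teardown logic is present but unconnected.
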(event `self.ReceiveBeginPlay`
  (bind _asbp_lobby_instance (cast `/Game/_Main/Menus/BP_LobbyInstance` (`GameplayStatics.GetGameInstance`)))
  (bind _output_get (set `self.Game Instance` _asbp_lobby_instance))
  (set `self.ScoreLimit` (`/Game/_Main/Menus/BP_LobbyInstance.ScoreLimit` _output_get))
  (set `self.MatchDuration` (`/Game/_Main/Menus/BP_LobbyInstance.MatchDuration` _output_get))
  (set `self.Num Players` (`/Game/_Main/Menus/BP_LobbyInstance.Num Players` _output_get)))

(event `Server_PlayerReady`
  (bind _playersready (`self.PlayersReady`))
  (bind _num_players (`self.Num Players`))
  (if (!= (`self.Num Players`) 0) :!label _label
    (bind _result (`/Engine/EditorBlueprintResources/StandardMacros.IncrementInt` _playersready)
      (:`  `
        (`KismetSystemLibrary.PrintString` (`KismetStringLibrary.Concat_StrStr` "Players Ready: " (`KismetStringLibrary.Conv_IntToString` _playersready)) true true (struct :`G` 0.66 :`B` 1.0 :`A` 1.0) 20.0)
        (`KismetSystemLibrary.PrintString` (`KismetStringLibrary.Concat_StrStr` "Players Expected: " (`KismetStringLibrary.Conv_IntToString` _num_players)) true true (struct :`G` 0.66 :`B` 1.0 :`A` 1.0) 20.0)
        (if (== _result _num_players)
          (bind _outactors (`GameplayStatics.GetAllActorsOfClass` "/Game/_Main/Game/Blueprints/Controllers/BP_FirstPersonController.BP_FirstPersonController_C"))
          (for _array_element _outactors
            (`/Game/_Main/Game/Blueprints/Controllers/BP_FirstPersonController.MC_StartCountdown` _array_element)))))
    (else
      (`KismetSystemLibrary.Delay` 0.2)
      (goto _label))))

(fn `CheckAllPlayersReady`)

(fn `Respawn`
  (returns (BestSpawn :type "Actor Object Reference"))
  (set `self.MaxDist` 0.0)
  (`KismetArrayLibrary.Array_Clear` (`self.AlivePlayers`))
  (bind _outactors (`GameplayStatics.GetAllActorsOfClass` "/Game/_Main/Game/Blueprints/Player/BP_Player.BP_Player_C"))
  (for _array_element _outactors
    (`/Engine/EditorBlueprintResources/StandardMacros.IsValid` _array_element
      (:`Is Valid`
        (if (> (`/Game/_Main/Game/Blueprints/Player/BP_Player.Health` _array_element) 0.0)
          (`KismetArrayLibrary.Array_Add` (`self.AlivePlayers`) _array_element)))))
  (bind _outactors_2 (`GameplayStatics.GetAllActorsOfClass` "/Script/Engine.PlayerStart"))
  (for _array_element_2 _outactors_2
    (for _array_element_3 (`self.AlivePlayers`)
      (bind _returnvalue (`KismetMathLibrary.VSize` (- (`self.K2_GetActorLocation` _array_element_3) (`self.K2_GetActorLocation` _array_element_2))))
      (if (> _returnvalue (`self.MaxDist`))
        (set `self.MaxDist` _returnvalue)
        (`KismetSystemLibrary.PrintString` "Max Dist Updated")
        (set `self.BestSpawn` _array_element_2))))
  (`KismetSystemLibrary.PrintString` (`KismetStringLibrary.Conv_DoubleToString` (`self.MaxDist`)))
  (return (`self.BestSpawn`)))

(fn `UserConstructionScript`)