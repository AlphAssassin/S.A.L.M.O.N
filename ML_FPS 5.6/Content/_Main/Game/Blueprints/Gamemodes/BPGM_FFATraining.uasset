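; Free-for-all game mode (FFA Training) that runs a match from ready-up to game over, then server-travels to Lobby.
; Loads match settings from the lobby game instance, tracks player controllers, and drops those with stale heartbeats.
; Once all players are ready, a countdown starts the match timer, whose expiry crowns top killers, including ties.
; Respawn picks the PlayerStart with the largest distance to any living player; kill handling is an empty stub.
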(event `self.ReceiveBeginPlay`
  (bind _players (`self.Players`))
  (`KismetArrayLibrary.Array_Clear` _players)
  (bind _asbp_first_person_controller (cast `/Game/_Main/Game/Blueprints/Controllers/BP_FirstPersonController` (`GameplayStatics.GetPlayerController` 0)))
  (`KismetArrayLibrary.Array_Add` _players _asbp_first_person_controller)
  (bind _asbp_lobby_instance (cast `/Game/_Main/Menus/BP_LobbyInstance` (`GameplayStatics.GetGameInstance`) :!label _label)
    (:`then`
      (bind _output_get (set `self.Game Instance` _asbp_lobby_instance))
      (set `self.ScoreLimit` (`/Game/_Main/Menus/BP_LobbyInstance.ScoreLimit` _output_get))
      (set `self.MatchDuration` (`/Game/_Main/Menus/BP_LobbyInstance.MatchDuration` _output_get))
      (set `self.Num Players` (`/Game/_Main/Menus/BP_LobbyInstance.Num Players` _output_get))
      (bind _asffagame_state (cast `/Game/_Main/Game/Blueprints/GameStates/FFAGameState` (`GameplayStatics.GetGameState`) :!label _label_2)
        (:`then`
          (set `self.FFAGame State` _asffagame_state)
          (`KismetSystemLibrary.K2_SetTimerDelegate` (delegate `CheckLastHeartbeats`) 2.0 true))
        (:`CastFailed`
          (`KismetSystemLibrary.DelayUntilNextTick`)
          (goto _label_2))))
    (:`CastFailed`
      (`KismetSystemLibrary.DelayUntilNextTick`)
      (goto _label))))

(event `CheckLastHeartbeats`
  (bind _outactors (`GameplayStatics.GetAllActorsOfClass` "/Game/_Main/Game/Blueprints/Controllers/BP_FirstPersonController.BP_FirstPersonController_C"))
  (for _array_element _outactors
    (if (> (- (`GameplayStatics.GetRealTimeSeconds`) (`/Game/_Main/Game/Blueprints/Controllers/BP_FirstPersonController.LastHearbeatTime` _array_element)) 5.0)
      (`self.PlayerDisconnect` _array_element))))

(event `self.K2_PostLogin`
  (params (NewPlayer :type "PlayerController Object Reference"))
  (bind _asbp_first_person_controller (cast `/Game/_Main/Game/Blueprints/Controllers/BP_FirstPersonController` NewPlayer))
  (bind _returnvalue (`KismetArrayLibrary.Array_Add` (`self.Players`) _asbp_first_person_controller))
  (`KismetSystemLibrary.PrintString` (`KismetStringLibrary.Conv_IntToString` _returnvalue))
  (`self.UpdateGameState`))

(event `Server_PlayerReady`
  (if (!= (`self.Num Players`) 0) :!label _label_3
    (bind _result (`/Engine/EditorBlueprintResources/StandardMacros.IncrementInt` (`self.PlayersReady`))
      (:`  `
        (if (== _result (`self.Num Players`))
          (bind _outactors (`GameplayStatics.GetAllActorsOfClass` "/Game/_Main/Game/Blueprints/Controllers/BP_FirstPersonController.BP_FirstPersonController_C"))
          (for _array_element _outactors
            (`/Game/_Main/Game/Blueprints/Controllers/BP_FirstPersonController.MC_StartCountdown` _array_element)
            (`KismetSystemLibrary.Delay` 3.0)
            (`self.FFAStart`)))))
    (else
      (`KismetSystemLibrary.Delay` 0.2)
      (goto _label_3))))

(event `PlayerDisconnect`
  (params (Controller :type "/Game/_Main/Game/Blueprints/Controllers/BP_FirstPersonController Object Reference"))
  (`KismetArrayLibrary.Array_RemoveItem` (`self.Players`) Controller)
  (bind _result (`/Engine/EditorBlueprintResources/StandardMacros.DecrementInt` (`self.Num Players`))
    (:`  `
      (`KismetSystemLibrary.PrintString` (`KismetStringLibrary.Conv_IntToString` _result))
      (`self.Server_PlayerReady`))))

(event `FFAStart`
  (bind _matchduration (`self.MatchDuration`))
  (bind _returnvalue (> _matchduration 0))
  (for _array_element (`self.Players`)
    (if _returnvalue
      (`/Game/_Main/Game/Blueprints/Controllers/BP_FirstPersonController.HUD_FFATimer` _array_element _matchduration)))
  (if _returnvalue
    (bind _returnvalue_2 (`KismetSystemLibrary.K2_SetTimer` null "MatchTimerInterval" 1.0 true))
    (set `self.MatchTimerHandle` _returnvalue_2)))

(event `MatchTimerInterval`
  (bind _result (`/Engine/EditorBlueprintResources/StandardMacros.DecrementInt` (`self.MatchDuration`))
    (:`  `
      (`/Game/_Main/Game/Blueprints/GameStates/FFAGameState.UpdateHud_Timer` (`self.FFAGame State`) _result)
      (if (== (`self.MatchDuration`) 0)
        (`KismetSystemLibrary.K2_ClearAndInvalidateTimerHandle` (`self.MatchTimerHandle`))
        ; True = End Match
        (bind _winners (`self.FindWinningPlayer`))
        (`self.GM_GameOver` false _winners)))))

(event `GM_GameOver`
  (params (IsScoreLimit :type Boolean) (Winner :type "Array of /Game/_Main/Game/Blueprints/Controllers/BP_FirstPersonController Object Reference"))
  (bind _players (`self.Players`))
  (`KismetSystemLibrary.PrintString` (`KismetStringLibrary.Conv_IntToString` (`KismetArrayLibrary.Array_Length` _players)) true true (struct :`G` 0.66 :`B` 1.0 :`A` 1.0) 15.0)
  (for _array_element _players
    (`/Game/_Main/Game/Blueprints/Controllers/BP_FirstPersonController.DisableControllerInput` _array_element)
    (`/Game/_Main/Game/Blueprints/Controllers/BP_FirstPersonController.UI Show GameOver` _array_element (!= (`KismetArrayLibrary.Array_Find` Winner _array_element) -1) IsScoreLimit)
    (set `self.IsGameOver` true))
  (`KismetSystemLibrary.Delay` 15.0)
  (`KismetSystemLibrary.ExecuteConsoleCommand` "servertravel Lobby" (`GameplayStatics.GetPlayerController` 0)))

(fn `CheckAllPlayersReady`)

(fn `FindWinningPlayer`
  (returns (Winners :type "Array of /Game/_Main/Game/Blueprints/Controllers/BP_FirstPersonController Object Reference"))
  (locals (Lcl_Kills :type "Array of Integer") (Lcl_AllWinnersFound :type Boolean) (Lcl_Winners :type "Array of /Game/_Main/Game/Blueprints/Controllers/BP_FirstPersonController Object Reference") (Lcl_WinKillCount :type Integer :default 0) (Lcl_Players :type "Array of /Game/_Main/Game/Blueprints/Controllers/BP_FirstPersonController Object Reference"))
  (bind _lcl_kills (`local.Lcl_Kills`))
  (bind (_indexofmaxvalue _maxvalue) (`KismetMathLibrary.MaxOfIntArray` (`local.Lcl_Kills`)))
  (bind _indexofmaxvalue_2 (`KismetMathLibrary.MaxOfIntArray` (`local.Lcl_Kills`)))
  (bind _asffagame_state (cast `/Game/_Main/Game/Blueprints/GameStates/FFAGameState` (`GameplayStatics.GetGameState`)))
  (for (_array_element _array_index) (`GameStateBase.PlayerArray` _asffagame_state)
    (bind _asffaplayer_state (cast `/Game/_Main/Game/Blueprints/GameStates/FFAPlayerState` _array_element))
    (`KismetArrayLibrary.Array_Set` (`local.Lcl_Kills`) _array_index (`/Game/_Main/Game/Blueprints/GameStates/FFAPlayerState.Kills` _asffaplayer_state) true)
    (bind _asbp_first_person_controller (cast `/Game/_Main/Game/Blueprints/Controllers/BP_FirstPersonController` (`PlayerState.GetPlayerController` _asffaplayer_state)))
    (`KismetArrayLibrary.Array_Set` (`local.Lcl_Players`) _array_index _asbp_first_person_controller true))
  (`KismetArrayLibrary.Array_Add` (`local.Lcl_Winners`) (`|GetArrayItem` (`local.Lcl_Players`) _indexofmaxvalue))
  (`KismetArrayLibrary.Array_Remove` (`local.Lcl_Players`) _indexofmaxvalue)
  (set `local.Lcl_WinKillCount` _maxvalue)
  (`KismetArrayLibrary.Array_Remove` (`local.Lcl_Kills`) _indexofmaxvalue)
  (while (not (`local.Lcl_AllWinnersFound`))
    (if (and (== (`local.Lcl_WinKillCount`) (`.MaxValue` (`KismetMathLibrary.MaxOfIntArray` _lcl_kills))) (> (`KismetArrayLibrary.Array_Length` _lcl_kills) 0))
      (`KismetArrayLibrary.Array_Add` (`local.Lcl_Winners`) (`|GetArrayItem` (`local.Lcl_Players`) _indexofmaxvalue_2))
      (`KismetArrayLibrary.Array_Remove` (`local.Lcl_Kills`) _indexofmaxvalue_2)
      (`KismetArrayLibrary.Array_Remove` (`local.Lcl_Players`) _indexofmaxvalue_2)
      (else
        (set `local.Lcl_AllWinnersFound` true))))
  (return (`local.Lcl_Winners`)))

(fn `GMPVP_KilledPlayer`
  (params (Killer :type "/Game/_Main/Game/Blueprints/Controllers/BP_FirstPersonController Object Reference") (Victim :type "/Game/_Main/Game/Blueprints/Controllers/BP_FirstPersonController Object Reference")))

(fn `Respawn`
  (returns (BestSpawn :type "Actor Object Reference"))
  (set `self.MaxDist` 0.0)
  (`KismetArrayLibrary.Array_Clear` (`self.AlivePlayers`))
  (bind _outactors (`GameplayStatics.GetAllActorsOfClass` "/Game/_Main/Game/Blueprints/Player/BP_Player.BP_Player_C"))
  (for _array_element _outactors
    (`/Engine/EditorBlueprintResources/StandardMacros.IsValid` _array_element
      (:`Is Valid`
        (if (> (`/Game/_Main/Game/Blueprints/Player/BP_Player.Health` _array_element) 0.0)
          (`KismetArrayLibrary.Array_Add` (`self.AlivePlayers`) _array_element)))))
  (bind _outactors_2 (`GameplayStatics.GetAllActorsOfClass` "/Script/Engine.PlayerStart"))
  (for _array_element_2 _outactors_2
    (for _array_element_3 (`self.AlivePlayers`)
      (bind _returnvalue (`KismetMathLibrary.VSize` (- (`self.K2_GetActorLocation` _array_element_3) (`self.K2_GetActorLocation` _array_element_2))))
      (if (> _returnvalue (`self.MaxDist`))
        (set `self.MaxDist` _returnvalue)
        (set `self.BestSpawn` _array_element_2))))
  (return (`self.BestSpawn`)))

(fn `UpdateGameState`
  (bind _ffagame_state (`self.FFAGame State`))
  (`/Engine/EditorBlueprintResources/StandardMacros.IsValid` _ffagame_state
    (:`Is Valid`
      (set `/Game/_Main/Game/Blueprints/GameStates/FFAGameState.MatchDuration` (`self.MatchDuration`) _ffagame_state)
      (set `/Game/_Main/Game/Blueprints/GameStates/FFAGameState.ScoreLimit` (`self.ScoreLimit`) _ffagame_state))))

(fn `UserConstructionScript`)