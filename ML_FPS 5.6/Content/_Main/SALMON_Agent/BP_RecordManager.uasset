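; BP_RecordManager is a Learning Agents manager Blueprint that records agent experience, with all work done on authority.
; BeginPlay creates the interactor, controller and recorder, then registers every BP_Agent with the Manager.
; Between Start and End Recording, Tick runs the controller and adds experience to the recorder.
; End Recording, also triggered by EndPlay, stops the recorder and saves the recording asset to a file under Saved/Recordings.
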(event `self.ReceiveBeginPlay`
  (`/Engine/EditorBlueprintResources/ActorMacros.Switch Has Authority`
    (:`Authority`
      (`|ExecutionSequence`
        (:`then_0`
          (bind _returnvalue (`LearningAgentsInteractor.MakeInteractor` (`self.Manager`) "/Game/_Main/SALMON_Agent/BP_AgentInteractor.BP_AgentInteractor_C"))
          (set `self.Interactor` _returnvalue))
        (:`then_1`
          (bind _returnvalue_2 (`LearningAgentsController.MakeController` (`self.Manager`) (`self.Interactor`) "/Game/_Main/SALMON_Agent/BP_AgentController.BP_AgentController_C"))
          (set `self.Controller` _returnvalue_2))
        (:`then_2`
          (bind _returnvalue_3 (`LearningAgentsRecorder.MakeRecorder` (`self.Manager`) (`self.Interactor`) "/Script/LearningAgentsTraining.LearningAgentsRecorder" "Recorder" (make `LearningAgentsRecorderPathSettings` (make `DirectoryPath` (`KismetStringLibrary.Concat_StrStr` (`KismetSystemLibrary.GetProjectSavedDirectory`) "Recordings/")) "LearningAgents") (`self.Recording Asset`) false))
          (set `self.Recorder` _returnvalue_3))
        (:`then_3`
          (bind _outactors (`GameplayStatics.GetAllActorsOfClass` "/Game/_Main/SALMON_Agent/BP_Agent.BP_Agent_C"))
          (bind _outagentids (`LearningAgentsManager.AddAgents` (`self.Manager`) _outactors))
          (set `self.Agent Ids` _outagentids))))))

(event `self.ReceiveTick`
  (params (DeltaSeconds :type "Float (single-precision)"))
  (if (`self.isRecording`)
    (`/Engine/EditorBlueprintResources/ActorMacros.Switch Has Authority`
      (:`Authority`
        (`LearningAgentsController.RunController` (`self.Controller`))
        (`LearningAgentsRecorder.AddExperience` (`self.Recorder`))
        (`KismetSystemLibrary.PrintString` (`KismetStringLibrary.Conv_IntToString` (`LearningAgentsManager.GetAgentNum` (`self.Manager`))))))))

(event `Start_Recording`
  (bind _recorder (`self.Recorder`))
  (`/Engine/EditorBlueprintResources/ActorMacros.Switch Has Authority`
    (:`Authority`
      (`LearningAgentsRecorder.BeginRecording` _recorder)
      (if (`LearningAgentsRecorder.IsRecording` _recorder)
        (`KismetSystemLibrary.PrintString` "Recording Started" true true (struct :`G` 0.66 :`B` 1.0 :`A` 1.0) 20.0)
        (set `self.isRecording` true)))))

(event `End_Recording`
  (`/Engine/EditorBlueprintResources/ActorMacros.Switch Has Authority` :!label _label
    (:`Authority`
      (`LearningAgentsRecorder.EndRecording` (`self.Recorder`))
      (`KismetSystemLibrary.PrintString` "Recording Ended" true true (struct :`G` 0.66 :`B` 1.0 :`A` 1.0) 20.0)
      (set `self.isRecording` false)
      (`LearningAgentsRecording.SaveRecordingToFile` (`self.Recording Asset`) (make `FilePath` (`KismetStringLibrary.Concat_StrStr` (`KismetSystemLibrary.GetProjectSavedDirectory`) "Recordings/Data.ueda"))))))

(event `self.ReceiveEndPlay`
  (params (EndPlayReason :type "EEndPlayReason Enum" :default "Destroyed"))
  (goto _label))

(fn `UserConstructionScript`)