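; Learning Agents interactor that defines what the BP_Agent shooter perceives and how it acts.
; Observations cover normalized enemy distance, facing dot product, health and ammo, line-of-sight, and agent-relative velocity directions of self and enemy.
; Actions drive movement, strafing, yaw, sensitivity-scaled pitch, firing and reloading on the pawn.
; An invalid nearest enemy only prints a warning; observation gathering still dereferences it.
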(fn `GatherAgentObservation`
  (params (InObservationObject :type "LearningAgentsObservationObject Object Reference") (AgentId :type Integer))
  (returns (OutObservationObjectElement :type "LearningAgentsObservationObjectElement Structure"))
  (locals (Agent :type "/Game/_Main/SALMON_Agent/BP_Agent Object Reference") (`Nearest Enemy` :type "Actor Object Reference") (DistToEnemy :type "Float (double-precision)" :default 0.0))
  (bind _agent (`local.Agent`))
  (bind _current_weapon (`/Game/_Main/SALMON_Agent/BP_Agent.Current Weapon` (`local.Agent`)))
  (bind _output_get (set `local.Agent` (`self.GetAgent` AgentId "/Game/_Main/SALMON_Agent/BP_Agent.BP_Agent_C")))
  (set `self.Can See Enemy` (`/Game/_Main/SALMON_Agent/BP_Agent.canSeeEnemy` _output_get))
  (bind _nearestenemy (`/Game/_Main/SALMON_Agent/BP_Agent.NearestEnemy` _output_get))
  (`/Engine/EditorBlueprintResources/StandardMacros.IsValid` _nearestenemy
    (:`Is Valid`
      _)
    (:`Is Not Valid`
      (`KismetSystemLibrary.PrintString` null "Invalid Enemy")))
  (set `local.Nearest Enemy` _nearestenemy)
  (bind _output_get_2 (set `local.DistToEnemy` (`/Game/_Main/SALMON_Agent/BP_Agent.DistToEnemy` _output_get)))
  (return (`LearningAgentsObservations.MakeStructObservation` (`local.InObservationObject`) (`|MakeMap` "EnemyDist" (`LearningAgentsObservations.MakeFloatObservation` (`local.InObservationObject`) (`KismetMathLibrary.FClamp` (/ _output_get_2 5000.0)) "EnemyDist" false null) "EnemyAngle" (`LearningAgentsObservations.MakeFloatObservation` (`local.InObservationObject`) (`KismetMathLibrary.Dot_VectorVector` (`Actor.GetActorForwardVector` (`local.Agent`)) (`KismetMathLibrary.Normal` (- (`Actor.K2_GetActorLocation` (`local.Nearest Enemy`)) (`Actor.K2_GetActorLocation` (`local.Agent`))))) "EnemyAngle" false null) "Health" (`LearningAgentsObservations.MakeFloatObservation` (`local.InObservationObject`) (`KismetMathLibrary.FClamp` (/ (`/Game/_Main/SALMON_Agent/BP_Agent.Health` _agent) (`/Game/_Main/SALMON_Agent/BP_Agent.MaxHealth` _agent))) "Health" false null) "CanSee" (`LearningAgentsObservations.MakeBoolObservation` (`local.InObservationObject`) (`self.Can See Enemy`) "CanSee" false null) "EnemyVel" (`LearningAgentsObservations.MakeDirectionObservation` (`local.InObservationObject`) (`KismetMathLibrary.Normal` (`Actor.GetVelocity` (`local.Nearest Enemy`))) (`Actor.GetTransform` (`local.Agent`)) "EnemyVel" false null) "SelfVel" (`LearningAgentsObservations.MakeDirectionObservation` (`local.InObservationObject`) (`KismetMathLibrary.Normal` (`Actor.GetVelocity` (`local.Agent`))) (`Actor.GetTransform` (`local.Agent`)) "SelfVel" false null) "Ammo" (`LearningAgentsObservations.MakeFloatObservation` (`local.InObservationObject`) (`KismetMathLibrary.FClamp` (/ (`/Game/_Main/Game/Blueprints/Weapons/BP_Weapon_Base.Ammo` _current_weapon) (`/Game/_Main/Game/Blueprints/Weapons/BP_Weapon_Base.MaxAmmo` _current_weapon))) "Ammo" false null) :!type "Name"))))

(fn `PerformAgentAction`
  (params (InActionObject :type "LearningAgentsActionObject Object Reference") (InActionObjectElement :type "LearningAgentsActionObjectElement Structure (by ref)") (AgentId :type Integer))
  (locals (agents :type "/Game/_Main/SALMON_Agent/BP_Agent Object Reference") (Actions :type "Map of Name to LearningAgentsActionObjectElement Structure"))
  (bind _agents (`local.agents`))
  (bind _agents_2 (`local.agents`))
  (bind _agents_3 (`local.agents`))
  (set `local.agents` (`self.GetAgent` AgentId "/Game/_Main/SALMON_Agent/BP_Agent.BP_Agent_C"))
  (bind _outelements (`LearningAgentsActions.GetStructAction` (`local.InActionObject`) (`local.InActionObjectElement`)))
  (set `local.Actions` _outelements)
  (`|ExecutionSequence`
    (:`then_0`
      (bind _outvalue (`LearningAgentsActions.GetFloatAction` (`local.InActionObject`) (`BlueprintMapLibrary.Map_Find` (`local.Actions`) "MoveForward") "MoveForward" false null))
      (`Pawn.AddMovementInput` _agents_2 (* _outvalue (`Actor.GetActorForwardVector` _agents_2)) 1.0 false))
    (:`then_1`
      (bind _outvalue_2 (`LearningAgentsActions.GetFloatAction` (`local.InActionObject`) (`BlueprintMapLibrary.Map_Find` (`local.Actions`) "Strafe") "Strafe" false null))
      (`Pawn.AddMovementInput` _agents (* _outvalue_2 (`Actor.GetActorRightVector` _agents)) 1.0 false))
    (:`then_2`
      (bind _outvalue_3 (`LearningAgentsActions.GetFloatAction` (`local.InActionObject`) (`BlueprintMapLibrary.Map_Find` (`local.Actions`) "Turn") "Turn" false null))
      (`Pawn.AddControllerYawInput` (`local.agents`) _outvalue_3))
    (:`then_3`
      (bind _outvalue_4 (`LearningAgentsActions.GetFloatAction` (`local.InActionObject`) (`BlueprintMapLibrary.Map_Find` (`local.Actions`) "Pitch") "Pitch" false null))
      (`Pawn.AddControllerPitchInput` (`local.agents`) (* _outvalue_4 (/ (`/Game/_Main/SALMON_Agent/BP_Agent.Vertical Sensitivity` (`local.agents`)) 2.5))))
    (:`then_4`
      (bind _boutvalue (`LearningAgentsActions.GetBoolAction` (`local.InActionObject`) (`BlueprintMapLibrary.Map_Find` (`local.Actions`) "Fire") "Fire" false null))
      (if _boutvalue
        (`/Game/_Main/SALMON_Agent/BP_Agent.Start_Fire` _agents_3)
        (else
          (`/Game/_Main/SALMON_Agent/BP_Agent.Stop_Fire` _agents_3))))
    (:`then_5`
      (bind _boutvalue_2 (`LearningAgentsActions.GetBoolAction` (`local.InActionObject`) (`BlueprintMapLibrary.Map_Find` (`local.Actions`) "Reload") "Reload" false null))
      (if _boutvalue_2
        (`/Game/_Main/SALMON_Agent/BP_Agent.Agent_Reload` (`local.agents`))))
    (:`then_6`
      (return))))

(fn `SpecifyAgentAction`
  (params (InActionSchema :type "LearningAgentsActionSchema Object Reference"))
  (returns (OutActionSchemaElement :type "LearningAgentsActionSchemaElement Structure"))
  (bind _output_get (set `self.ActMoveForward` (`LearningAgentsActions.SpecifyFloatAction` InActionSchema 1.0 "MoveForward")))
  (bind _output_get_2 (set `self.ActStrafe` (`LearningAgentsActions.SpecifyFloatAction` InActionSchema 1.0 "Strafe")))
  (bind _output_get_3 (set `self.ActTurn` (`LearningAgentsActions.SpecifyFloatAction` InActionSchema 1.0 "Turn")))
  (bind _output_get_4 (set `self.ActPitch` (`LearningAgentsActions.SpecifyFloatAction` InActionSchema 1.0 "Pitch")))
  (bind _output_get_5 (set `self.ActFire` (`LearningAgentsActions.SpecifyBoolAction` InActionSchema 0.5 "Fire")))
  (bind _output_get_6 (set `self.ActReload` (`LearningAgentsActions.SpecifyBoolAction` InActionSchema 0.5 "Reload")))
  (return (`LearningAgentsActions.SpecifyStructAction` InActionSchema (`|MakeMap` "MoveForward" _output_get "Strafe" _output_get_2 "Turn" _output_get_3 "Pitch" _output_get_4 "Fire" _output_get_5 "Reload" _output_get_6 :!type "Name"))))

(fn `SpecifyAgentObservation`
  (params (InObservationSchema :type "LearningAgentsObservationSchema Object Reference"))
  (returns (OutObservationSchemaElement :type "LearningAgentsObservationSchemaElement Structure"))
  (bind _output_get (set `self.ObsEnemyDist` (`LearningAgentsObservations.SpecifyFloatObservation` InObservationSchema 1.0 "EnemyDist")))
  (bind _output_get_2 (set `self.ObsEnemyAngle` (`LearningAgentsObservations.SpecifyFloatObservation` InObservationSchema 1.0 "EnemyAngle")))
  (bind _output_get_3 (set `self.ObsHealth` (`LearningAgentsObservations.SpecifyFloatObservation` InObservationSchema 1.0 "Health")))
  (bind _output_get_4 (set `self.ObsCanSee` (`LearningAgentsObservations.SpecifyBoolObservation` InObservationSchema "CanSee")))
  (bind _output_get_5 (set `self.ObsEnemyVel` (`LearningAgentsObservations.SpecifyDirectionObservation` InObservationSchema "EnemyVel")))
  (bind _output_get_6 (set `self.ObsSelfVel` (`LearningAgentsObservations.SpecifyDirectionObservation` InObservationSchema "SelfVel")))
  (bind _output_get_7 (set `self.ObsAmmo` (`LearningAgentsObservations.SpecifyFloatObservation` InObservationSchema 1.0 "Ammo")))
  (return (`LearningAgentsObservations.SpecifyStructObservation` InObservationSchema (`|MakeMap` "EnemyDist" _output_get "EnemyAngle" _output_get_2 "Health" _output_get_3 "CanSee" _output_get_4 "EnemyVel" _output_get_5 "SelfVel" _output_get_6 "Ammo" _output_get_7 :!type "Name"))))