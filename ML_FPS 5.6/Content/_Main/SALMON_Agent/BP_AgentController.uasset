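; BP_AgentController is a Learning Agents controller that turns a player character's inputs into an agent action, so human play can stand in for the agent's decisions.
; It resolves the BP_Agent by ID, then reads the input values on its linked PlayerChar.
; Movement and look inputs become float actions and Fire and Reload become bool actions, all packed into one named struct action.
; The observation inputs are unused.
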(fn `EvaluateAgentController`
  (params (InActionObject :type "LearningAgentsActionObject Object Reference") (InObservationObject :type "LearningAgentsObservationObject Object Reference") (InObservationObjectElement :type "LearningAgentsObservationObjectElement Structure (by ref)") (AgentId :type Integer))
  (returns (OutActionObjectElement :type "LearningAgentsActionObjectElement Structure"))
  (locals (Player :type "/Game/_Main/Game/Blueprints/Player/BP_Player Object Reference") (`Agent Char` :type "/Game/_Main/SALMON_Agent/BP_Agent Object Reference"))
  (bind _player (`local.Player`))
  (bind _player_2 (`local.Player`))
  (bind _player_3 (`local.Player`))
  (bind _output_get (set `local.Agent Char` (`self.GetAgent` AgentId "/Game/_Main/SALMON_Agent/BP_Agent.BP_Agent_C")))
  (set `local.Player` (`/Game/_Main/SALMON_Agent/BP_Agent.PlayerChar` _output_get))
  (return (`LearningAgentsActions.MakeStructAction` (`local.InActionObject`) (`|MakeMap` "MoveForward" (`LearningAgentsActions.MakeFloatAction` (`local.InActionObject`) (`/Game/_Main/Game/Blueprints/Player/BP_Player.InputMoveForward` _player_2) "MoveForward" false null) "Strafe" (`LearningAgentsActions.MakeFloatAction` (`local.InActionObject`) (`/Game/_Main/Game/Blueprints/Player/BP_Player.InputStrafe` _player_2) "Strafe" false null) "Turn" (`LearningAgentsActions.MakeFloatAction` (`local.InActionObject`) (`/Game/_Main/Game/Blueprints/Player/BP_Player.InputTurn` _player_3) "Turn" false null) "Pitch" (`LearningAgentsActions.MakeFloatAction` (`local.InActionObject`) (`/Game/_Main/Game/Blueprints/Player/BP_Player.InputLookUp` _player_3) "Pitch" false null) "Fire" (`LearningAgentsActions.MakeBoolAction` (`local.InActionObject`) (`/Game/_Main/Game/Blueprints/Player/BP_Player.InputFire` _player) "Fire" false null) "Reload" (`LearningAgentsActions.MakeBoolAction` (`local.InActionObject`) (`/Game/_Main/Game/Blueprints/Player/BP_Player.InputReload` _player) "Reload" false null) :!type "Name"))))