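; BP_Dummy is a damageable dummy that ragdolls when killed and respawns where it began play.
; Point damage lowers Health; at zero, Die enables physics simulation and the Ragdoll collision profile on the skeletal mesh.
; Tick polls for zero Health and, after a three-second Delay, calls Respawn to restore transform, collision, Health and the ABP_Player animation Blueprint.
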(event `self.ReceiveBeginPlay`
  (set `self.SpawnLocation` (`self.K2_GetActorLocation`))
  (set `self.SpawnRotation` (`self.K2_GetActorRotation`)))

(event `self.ReceiveTick`
  (params (DeltaSeconds :type "Float (single-precision)"))
  (if (<= (`self.Health`) 0.0)
    (`self.Die`)
    (`KismetSystemLibrary.Delay` 3.0)
    (`self.Respawn`)))

(event `self.ReceivePointDamage`
  (params (Damage :type "Float (single-precision)") (DamageType :type "DamageType Object Reference") (HitLocation :type "Vector Structure") (HitNormal :type "Vector Structure") (HitComponent :type "PrimitiveComponent Object Reference") (BoneName :type Name) (ShotFromDirection :type "Vector Structure") (InstigatedBy :type "Controller Object Reference") (DamageCauser :type "Actor Object Reference") (HitInfo :type "HitResult Structure (by ref)"))
  (bind _output_get (set `self.Health` (- (`self.Health`) Damage)))
  (if (<= _output_get 0.0)
    (`self.Die`)
    (else
      (`KismetSystemLibrary.PrintString` "Dummy took damage"))))

(fn `Die`
  (bind _skeletalmesh (`self.SkeletalMesh`))
  (`PrimitiveComponent.SetSimulatePhysics` _skeletalmesh true)
  (`PrimitiveComponent.SetCollisionProfileName` _skeletalmesh "Ragdoll" true)
  (return))

(fn `Respawn`
  (bind _skeletalmesh (`self.SkeletalMesh`))
  (`self.K2_SetActorLocationAndRotation` (`self.SpawnLocation`) (`self.SpawnRotation`) true)
  (`PrimitiveComponent.SetSimulatePhysics` _skeletalmesh false)
  (`PrimitiveComponent.SetCollisionProfileName` _skeletalmesh "Pawn" true)
  (`SceneComponent.ResetRelativeTransform` (`self.SkeletalMesh`))
  (set `self.Health` (`self.MaxHealth`))
  (`SkeletalMeshComponent.SetAnimationMode` (`self.SkeletalMesh`) "AnimationBlueprint" true)
  (`SkeletalMeshComponent.SetAnimInstanceClass` (`self.SkeletalMesh`) "/Game/_Main/Blueprints/Player/Animations/ABP_Player.ABP_Player_C"))

(fn `UserConstructionScript`)