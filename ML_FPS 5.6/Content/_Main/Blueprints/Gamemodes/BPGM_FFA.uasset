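; Free-for-all game mode Blueprint whose Respawn function picks a PlayerStart away from living players.
; It rebuilds the list of BP_Player actors with health above zero, then measures each one's distance to every PlayerStart.
; The start from the farthest single player-to-start pair wins, rather than the one farthest from its nearest player.
; MaxDist is not reset within the function, and the event graph is empty.
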(fn `Respawn`
  (returns (BestSpawn :type "Actor Object Reference"))
  (`KismetArrayLibrary.Array_Clear` (`self.AlivePlayers`))
  (bind _outactors (`GameplayStatics.GetAllActorsOfClass` "/Game/_Main/Blueprints/Player/BP_Player.BP_Player_C"))
  (for _array_element _outactors
    (`/Engine/EditorBlueprintResources/StandardMacros.IsValid` _array_element
      (:`Is Valid`
        (if (> (`/Game/_Main/Blueprints/Player/BP_Player.Health` _array_element) 0.0)
          (`KismetArrayLibrary.Array_Add` (`self.AlivePlayers`) _array_element)))))
  (bind _outactors_2 (`GameplayStatics.GetAllActorsOfClass` "/Script/Engine.PlayerStart"))
  (for _array_element_2 _outactors_2
    (for _array_element_3 (`self.AlivePlayers`)
      (bind _returnvalue (`KismetMathLibrary.VSize` (- (`self.K2_GetActorLocation` _array_element_3) (`self.K2_GetActorLocation` _array_element_2))))
      (if (> _returnvalue (`self.MaxDist`))
        (set `self.MaxDist` _returnvalue)
        (set `self.BestSpawn` _array_element_2))))
  (return (`self.BestSpawn`)))

(fn `UserConstructionScript`)