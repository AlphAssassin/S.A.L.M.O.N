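; Base bullet actor for weapons that damages what it hits and then disappears.
; On spawn, its Collider is set to ignore the owner and instigator while moving.
; When the Collider hits, the bullet calls destroy on itself first, then applies its Damage value to the other actor if that actor is valid and not the owner.
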(event `self.ReceiveBeginPlay`
  (`PrimitiveComponent.IgnoreActorWhenMoving` (`self.Collider`) (`self.GetOwner`) true)
  (`PrimitiveComponent.IgnoreActorWhenMoving` (`self.Collider`) (`self.GetInstigator`) true))

(event `self.ReceiveHit`
  (params (MyComp :type "PrimitiveComponent Object Reference") (Other :type "Actor Object Reference") (OtherComp :type "PrimitiveComponent Object Reference") (bSelfMoved :type Boolean) (HitLocation :type "Vector Structure") (HitNormal :type "Vector Structure") (NormalImpulse :type "Vector Structure") (Hit :type "HitResult Structure (by ref)")))

(event `self.Collider.OnComponentHit`
  (params (HitComponent :type "PrimitiveComponent Object Reference") (OtherActor :type "Actor Object Reference") (OtherComp :type "PrimitiveComponent Object Reference") (NormalImpulse :type "Vector Structure") (Hit :type "HitResult Structure (by ref)"))
  (`self.K2_DestroyActor`)
  (`/Engine/EditorBlueprintResources/StandardMacros.IsValid` OtherActor
    (:`Is Valid`
      (if (!= OtherActor (`self.GetOwner`))
        (`GameplayStatics.ApplyDamage` OtherActor (`self.Damage`))))))

(fn `UserConstructionScript`)