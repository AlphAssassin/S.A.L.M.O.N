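; Base weapon Blueprint for guns attached to BP_Player, handling firing, ammo and reloading with server/client event pairs.
; Server fire traces through the player's crosshair component, adds spread and, on a hit, spawns a bullet from the muzzle toward it.
; Client fire plays muzzle effect and sound and decrements ammo.
; Reload triggers montages on both player meshes, while the server refills ammo after the montage's length.
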(event `Server_Fire`
  (bind _returnvalue (`SceneComponent.GetSocketLocation` (`self.WeaponMesh`) (`self.MuzzleSocket`)))
  (if (> (`self.Ammo`) 0)
    (bind _asbp_player (cast `/Game/_Main/Blueprints/Player/BP_Player` (`ActorComponent.GetOwner` (`SceneComponent.GetAttachParent` (`self.DefaultSceneRoot`)))))
    (bind _ct_cmpt_crosshair (`/Game/_Main/Blueprints/Player/BP_Player.CT_Cmpt_Crosshair` _asbp_player))
    (bind (_outlocation _outrotation) (`self.GetActorEyesViewPoint` _asbp_player))
    (bind (_outhit _returnvalue_2) (`/Game/CT_Components/CrosshairSystem/Components/CT_Cmpt_Crosshair.LineTraceByChannel` :`self` _ct_cmpt_crosshair :`StartPoint` (`KismetMathLibrary.MakeTransform` _outlocation _outrotation) :`DrawDebugType` "ForDuration"))
    (`/Game/CT_Components/CrosshairSystem/Components/CT_Cmpt_Crosshair.AddDynamicSpread` _ct_cmpt_crosshair 20.0 0.5)
    (if _returnvalue_2
      (`|SpawnActorFromClass` (`self.BulletClass`) (`KismetMathLibrary.MakeTransform` _returnvalue (`KismetMathLibrary.MakeRotFromX` (- (`.Location` (`GameplayStatics.BreakHitResult` _outhit)) _returnvalue))) "Undefined" "MultiplyWithRoot" (`GameplayStatics.GetPlayerController` 0) (`GameplayStatics.GetPlayerCharacter` 0)))))

(event `Client Fire`
  ;[1 1 1] Spawn Emitter and play shot sound
  (`GameplayStatics.SpawnEmitterAttached` (`self.MuzzleEffect`) null (`self.MuzzleSocket`))
  (`GameplayStatics.PlaySoundAtLocation` (`self.Sound`) (0.0 0.0 0.0) (struct) 1.0 1.0 0.0 null null null null)
  (set `self.Ammo` (- (`self.Ammo`) 1)))

(event `Client_Reload`
  (bind _montage_to_play (`self.Montage to Play`))
  (bind _asbp_player (cast `/Game/_Main/Blueprints/Player/BP_Player` (`ActorComponent.GetOwner` (`SceneComponent.GetAttachParent` (`self.DefaultSceneRoot`)))))
  (`|PlayMontage` (`Character.Mesh` _asbp_player) _montage_to_play 1.0 0.0 "None" false
    (:`then`
      (`|PlayMontage` (`/Game/_Main/Blueprints/Player/BP_Player.OtherPlayer` _asbp_player) _montage_to_play 1.0 0.0 "None" false))
    (:`OnCompleted`
      (`KismetSystemLibrary.PrintString` "Finish Reload"))))

(event `Server_Reload`
  (if (< (`self.Ammo`) (`self.MaxAmmo`))
    (`self.Client_Reload`)
    (`KismetSystemLibrary.Delay` (`AnimationAsset.GetPlayLength` (`self.Montage to Play`)))
    (set `self.Ammo` (`self.MaxAmmo`))))

(fn `FireWeapon`
  (`self.Server_Fire`)
  (`self.Client Fire`))

(fn `OnRep_Ammo`)

(fn `Reload`
  (if (< (`self.Ammo`) (`self.MaxAmmo`))
    (`self.Server_Reload`)))

(fn `UserConstructionScript`)