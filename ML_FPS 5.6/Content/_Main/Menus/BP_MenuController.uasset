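; BP_MenuController is the menu and lobby player controller, handling UI-only input, the lobby widget and leaving a session for MainMenu.
; InitSetup loads or creates the saved player profile, then passes it through ServerUpdateLobby to BPGM_Lobby to trigger a lobby update.
; UpdatePlayerNames hands the profiles to the lobby widget's ClearPlayerNames.
; Tick toggles cursor visibility from MouseX input down time.
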(event `self.ReceiveBeginPlay`
  (if (`self.IsLocalController`)
    (set `self.bShowMouseCursor` true)
    (`WidgetBlueprintLibrary.SetInputMode_UIOnlyEx` self null "LockInFullscreen")))

(event `self.ReceiveTick`
  (params (DeltaSeconds :type "Float (single-precision)"))
  (if (> (`self.GetInputKeyTimeDown` "MouseX") 0.0)
    (set `self.bShowMouseCursor` true)
    (else
      (set `self.bShowMouseCursor` false))))

(event `EndClientSession`
  (`DestroySessionCallbackProxy.DestroySession` self
    (:`then`
      (`GameplayStatics.OpenLevel` "MainMenu"))))

(event `Create Lobby Menu`
  (`self.UI_ShowLobbyMenu`))

(event `InitSetup`
  (`self.LoadSavedProfile`)
  (`self.ServerUpdateLobby` (`self.Player Profile`)))

(event `ServerUpdateLobby`
  (params (PlayerProfile :type "/Game/_Main/PlayerName/S_PlayerProfile Structure"))
  (`KismetSystemLibrary.PrintText` (`.PlayerName_2_EB8B0EAE472EF0E8B03D6C9F55C6C98E` (break `/Game/_Main/PlayerName/S_PlayerProfile` PlayerProfile)))
  (set `self.Player Profile` PlayerProfile)
  (bind _asbpgm_lobby (cast `/Game/_Main/Menus/BPGM_Lobby` (`GameplayStatics.GetGameMode`)))
  (`/Game/_Main/Menus/BPGM_Lobby.UpdateLobby` _asbpgm_lobby true))

(event `UpdatePlayerNames`
  (params (PlayerProfiles :type "Array of /Game/_Main/PlayerName/S_PlayerProfile Structure"))
  (bind _lobbymenu (`self.LobbyMenu`))
  (`/Engine/EditorBlueprintResources/StandardMacros.IsValid` _lobbymenu
    (:`Is Valid`
      (`/Game/_Main/Menus/WBP_Lobby.ClearPlayerNames` _lobbymenu PlayerProfiles)
      (`KismetSystemLibrary.Delay` 5.0))))

(fn `LoadSavedProfile`
  (locals (Lcl_SlotName :type String :default "PlayerProfileSlot"))
  (bind _returnvalue (`GameplayStatics.DoesSaveGameExist` (`local.Lcl_SlotName`)))
  (if (not _returnvalue)
    (bind _returnvalue_2 (`GameplayStatics.CreateSaveGameObject` "/Game/_Main/PlayerName/SG_PlayerProfile.SG_PlayerProfile_C"))
    (`GameplayStatics.SaveGameToSlot` _returnvalue_2 (`local.Lcl_SlotName`)))
  (bind _returnvalue_3 (`GameplayStatics.LoadGameFromSlot` (`local.Lcl_SlotName`)))
  (bind _assg_player_profile (cast `/Game/_Main/PlayerName/SG_PlayerProfile` _returnvalue_3))
  (set `self.Player Profile` (`/Game/_Main/PlayerName/SG_PlayerProfile.PlayerProfile` _assg_player_profile))
  (return))

(fn `UI_ShowLobbyMenu`
  (`/Engine/EditorBlueprintResources/StandardMacros.IsValid` (`self.LobbyMenu`)
    (:`Is Valid`
      _)
    (:`Is Not Valid`
      (bind _returnvalue (`|CreateWidget` "/Game/_Main/Menus/WBP_Lobby.WBP_Lobby_C" (`GameplayStatics.GetPlayerController` 0)))
      (set `self.LobbyMenu` _returnvalue)))
  (`UserWidget.AddToViewport` (`self.LobbyMenu`) 0)
  (return))

(fn `UserConstructionScript`)