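; BP_BulletBase is a bullet actor, named as a base for weapon projectiles, that damages BP_Dummy targets on impact.
; Its Collider hit event casts the hit actor to BP_Dummy and subtracts Damage directly from that dummy's Health variable.
; The bullet destroys itself on any valid hit, with debug prints of the actor's name and "Damage Applied", the latter appearing even for non-dummy hits.
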(event `self.ReceiveHit`
  (params (MyComp :type "PrimitiveComponent Object Reference") (Other :type "Actor Object Reference") (OtherComp :type "PrimitiveComponent Object Reference") (bSelfMoved :type Boolean) (HitLocation :type "Vector Structure") (HitNormal :type "Vector Structure") (NormalImpulse :type "Vector Structure") (Hit :type "HitResult Structure (by ref)")))

(event `self.Collider.OnComponentHit`
  (params (HitComponent :type "PrimitiveComponent Object Reference") (OtherActor :type "Actor Object Reference") (OtherComp :type "PrimitiveComponent Object Reference") (NormalImpulse :type "Vector Structure") (Hit :type "HitResult Structure (by ref)"))
  (`KismetSystemLibrary.PrintString` (`KismetSystemLibrary.GetDisplayName` OtherActor))
  (`/Engine/EditorBlueprintResources/StandardMacros.IsValid` OtherActor
    (:`Is Valid`
      (bind _asbp_dummy (cast `/Game/_Main/Blueprints/Player/BP_Dummy` OtherActor)
        (:`then`
          (set `/Game/_Main/Blueprints/Player/BP_Dummy.Health` (- (`/Game/_Main/Blueprints/Player/BP_Dummy.Health` _asbp_dummy) (`self.Damage`)) _asbp_dummy))
        (:`CastFailed`
          _))
      (`self.K2_DestroyActor`)
      (`KismetSystemLibrary.PrintString` "Damage Applied"))))

(fn `UserConstructionScript`)