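; Base weapon Blueprint that fires projectiles and tracks ammo.
; The IA_Shoot input action calls FireWeapon, which checks for remaining Ammo, spawns BulletClass at the weapon mesh's MuzzleSocket transform and decrements the count.
; Nodes for a muzzle emitter and shot sound exist in FireWeapon but are unconnected, so they never run.
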(event `EnhancedInput|/Game/_Main/Blueprints/Input/Actions/IA_Shoot`
  (params (ActionValue :type Boolean) (ElapsedSeconds :type "Float (double-precision)") (TriggeredSeconds :type "Float (double-precision)") (InputAction :type "InputAction Object Reference" :default "/Game/_Main/Blueprints/Input/Actions/IA_Shoot.IA_Shoot"))
  (:`Triggered`
    (`self.FireWeapon`)))

(fn `FireWeapon`
  (if (> (`self.Ammo`) 0)
    (`|SpawnActorFromClass` (`self.BulletClass`) (`SceneComponent.GetSocketTransform` (`self.WeaponMesh`) (`self.MuzzleSocket`) "RTS_World") "Undefined" "MultiplyWithRoot" null null)
    (set `self.Ammo` (- (`self.Ammo`) 1))))

(fn `UserConstructionScript`)