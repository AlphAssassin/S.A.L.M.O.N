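; Character selection Blueprint that lets the player pick a soldier skeletal mesh and two materials, with the mouse cursor shown.
; Events swap the mesh from a character array and set material slots 0 and 1.
; Choices save to a CharacterSelection_Save slot, reloaded on BeginPlay if it exists or via ResetOnExit.
; A timeline-driven RInterpTo eases the mesh yaw when resetting rotation on exit.
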(event `Character_Event12`
  (params (SK_Integer :type Integer))
  ;[1 1 1 1 30] Character Selection
  (`SkinnedMeshComponent.SetSkinnedAssetAndUpdate` (`self.Mesh`) (`|GetArrayItem` (`self.Characters`) SK_Integer) true))

(event `Material01`
  (params (Material_01 :type "MaterialInterface Object Reference"))
  ;[1 1 1 1 30] Material 01 Selection
  (bind _output_get (set `self.Material_01_Reference` Material_01))
  (`PrimitiveComponent.SetMaterial` (`self.Mesh`) 0 _output_get))

(event `Material02`
  (params (Material_02 :type "MaterialInterface Object Reference"))
  ;[1 1 1 1 30] Material 02 Selection
  (bind _output_get (set `self.Material_02_Reference` Material_02))
  (`PrimitiveComponent.SetMaterial` (`self.Mesh`) 1 _output_get))

(event `Save`
  ;[1 1 1 1 30] Save
  (bind _returnvalue (`GameplayStatics.CreateSaveGameObject` "/Game/LowPoly_Soldiers/BluePrints/CharacterSelection_Save.CharacterSelection_Save_C"))
  (bind _output_get (set `self.SaveGameClass` _returnvalue))
  (bind _ascharacter_selection_save (cast `/Game/LowPoly_Soldiers/BluePrints/CharacterSelection_Save` _output_get))
  (set `/Game/LowPoly_Soldiers/BluePrints/CharacterSelection_Save.Material_02_Save` (`self.Material_02_Reference`) _ascharacter_selection_save)
  (set `/Game/LowPoly_Soldiers/BluePrints/CharacterSelection_Save.Material_01_Save` (`self.Material_01_Reference`) _ascharacter_selection_save)
  (set `/Game/LowPoly_Soldiers/BluePrints/CharacterSelection_Save.Character_Integer` (`self.Character Integer`) _ascharacter_selection_save)
  (`GameplayStatics.SaveGameToSlot` (`self.SaveGameClass`) (`self.SaveGame_Var`)))

(event `ResetOnExit`
  (bind _mesh (`self.Mesh`))
  ;[1 1 1 1 30] Load
  (bind _returnvalue (`GameplayStatics.LoadGameFromSlot` (`self.SaveGame_Var`) :!label _label))
  (bind _output_get (set `self.SaveGameClass` _returnvalue))
  (bind _ascharacter_selection_save (cast `/Game/LowPoly_Soldiers/BluePrints/CharacterSelection_Save` _output_get))
  (`|ExecutionSequence`
    (:`then_0`
      (bind _output_get_2 (set `self.Character Integer` (`/Game/LowPoly_Soldiers/BluePrints/CharacterSelection_Save.Character_Integer` _ascharacter_selection_save)))
      (`self.Character_Event12` _output_get_2))
    (:`then_1`
      (bind _output_get_3 (set `self.Material_01_Reference` (`/Game/LowPoly_Soldiers/BluePrints/CharacterSelection_Save.Material_01_Save` _ascharacter_selection_save)))
      (`PrimitiveComponent.SetMaterial` _mesh 0 _output_get_3))
    (:`then_2`
      (bind _output_get_4 (set `self.Material_02_Reference` (`/Game/LowPoly_Soldiers/BluePrints/CharacterSelection_Save.Material_02_Save` _ascharacter_selection_save)))
      (`PrimitiveComponent.SetMaterial` _mesh 1 _output_get_4))))

(event `self.ReceiveBeginPlay`
  ;[1 1 1 1 30] Load
  (set `PlayerController.bShowMouseCursor` true (`GameplayStatics.GetPlayerController` 0))
  (bind _returnvalue (`GameplayStatics.DoesSaveGameExist` (`self.SaveGame_Var`)))
  (if _returnvalue
    (goto _label)))

(event `ResetRotationOnExit`
  ;[1 1 1 1 30] Reset Rotation on Exit
  (bind (_direction _resetrotation) (`Timeline|Timeline_0` :!via `PlayFromStart`)
    (:`Update`
      (bind (_returnvalue_roll _returnvalue_pitch _returnvalue_yaw) (`KismetMathLibrary.BreakRotator` (`KismetMathLibrary.RInterpTo` (`KismetMathLibrary.MakeRotator` 0.0 0.0 (`self.CharacterRotation`)) (struct) _resetrotation 0.1)))
      (bind _output_get (set `self.CharacterRotation` _returnvalue_yaw))
      (`SceneComponent.K2_SetWorldRotation` (`self.Mesh`) (`KismetMathLibrary.MakeRotator` 0.0 0.0 _output_get) false false))))

(fn `UserConstructionScript`)